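; BP_HealthPack is a pickup actor that restores health to the player.
; On overlap with a BP_Player it calls IncreaseHealth by a fixed amount and destroys itself.
; It caches the player pawn at BeginPlay and checks distance to it every Tick, destroying itself once the player is far away.
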(event `self.ReceiveBeginPlay`
  (bind _asbp_player (cast `/Game/InfiniteMatrix/Blueprints/BP_Player` (`GameplayStatics.GetPlayerPawn` 0)))
  (bind _output_get (set `self.PlayerReference` _asbp_player)))

(event `self.ReceiveActorBeginOverlap`
  (params (OtherActor :type "Actor Object Reference"))
  (bind _asbp_player (cast `/Game/InfiniteMatrix/Blueprints/BP_Player` OtherActor))
  (`/Game/InfiniteMatrix/Blueprints/BP_Player.IncreaseHealth` _asbp_player 1.0)
  (`self.K2_DestroyActor`))

(event `self.ReceiveTick`
  (params (DeltaSeconds :type "Float (single-precision)"))
  (if (> (`KismetMathLibrary.VSize` (- (`self.K2_GetActorLocation`) (`self.K2_GetActorLocation` (stale `self.ReceiveBeginPlay` _output_get)))) 10000.0)
    (`self.K2_DestroyActor`)))

(fn `UserConstructionScript`)